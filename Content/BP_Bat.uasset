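; BP_Bat is a player-controlled bat that winds up and swings, likely for hitting a piñata.
; Holding PlayerAction plays the Hold timeline to yaw the static mesh back or round; releasing stops it and plays the Huyak swing timeline.
; Swing amplitude is scaled through a Lerp on Hold's remaining time, so a longer hold gives a bigger swing.
; Hits on BP_Candy fire the HitPinjata dispatcher.
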(event `InputAction|PlayerAction` :overrideparent false
  (params (Key :type "Key Structure"))
  (bind _hold (`self.Hold`))
  (bind _staticmesh (`self.StaticMesh`))
  (:`Pressed`
    (`KismetSystemLibrary.PrintString` "Hold")
    (bind (_direction _hold_2) (`Timeline|Hold` :!via `PlayFromStart`)
      (:`Update`
        (`SceneComponent.K2_SetRelativeRotation` _staticmesh (`KismetMathLibrary.MakeRotator` -60.0 0.0 (* _hold_2 60.0)) false false))))
  (:`Released`
    (`KismetSystemLibrary.PrintString` "Hello")
    (`TimelineComponent.Stop` (`self.Hold`))
    (bind (_direction_2 _hit) (`Timeline|Huyak` :!via `PlayFromStart`)
      (:`Update`
        (`SceneComponent.K2_SetRelativeRotation` _staticmesh (`KismetMathLibrary.MakeRotator` -60.0 0.0 (* _hit 80.0 (`KismetMathLibrary.Lerp` 1.0 0.1 (* (- (`TimelineComponent.GetTimelineLength` _hold) (`TimelineComponent.GetPlaybackPosition` _hold)) 2.0)))) false false)))))

(event `self.ReceiveHit`
  (params (MyComp :type "PrimitiveComponent Object Reference") (Other :type "Actor Object Reference") (OtherComp :type "PrimitiveComponent Object Reference") (bSelfMoved :type Boolean) (HitLocation :type "Vector Structure") (HitNormal :type "Vector Structure") (NormalImpulse :type "Vector Structure") (Hit :type "HitResult Structure (by ref)"))
  (cast `/Game/BP_Candy` Other)
  (`self.HitPinjata`))

(fn `UserConstructionScript`)