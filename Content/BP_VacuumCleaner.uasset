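; Vacuum cleaner actor that sucks up nearby candy and reports each piece collected to BP_GameMode.
; Every Tick it scans all BP_Candy actors and pulls those within MaxDragRadius toward its Magnet, faster as they get closer, scaled by frame pace.
; Candy inside TargetDragRadius is destroyed with an eat sound and triggers a timeline that pulses the CandyBag's scale and emissive material.
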(event `self.ReceiveBeginPlay`
  (set `self.BagScale` (`SceneComponent.RelativeScale3D` (`self.CandyBag`))))

(event `self.ReceiveTick`
  (params (DeltaSeconds :type "Float (single-precision)"))
  (bind _outactors (`GameplayStatics.GetAllActorsOfClass` "/Game/BP_Candy.BP_Candy_C"))
  (for _array_element _outactors
    (bind _candy1 (`/Game/BP_Candy.Candy1` _array_element))
    (bind _returnvalue (- (`SceneComponent.K2_GetComponentLocation` (`self.Magnet`)) (`SceneComponent.K2_GetComponentLocation` _candy1)))
    (bind _returnvalue_2 (`KismetMathLibrary.VSize` _returnvalue))
    (if (< _returnvalue_2 (`self.MaxDragRadius`))
      (if (< _returnvalue_2 (`self.TargetDragRadius`))
        (`self.K2_DestroyActor` _array_element)
        (`GameplayStatics.PlaySound2D` "/Game/Sound/Eat.Eat" 1.0 1.0 0.0 null null)
        (bind _asbp_game_mode (cast `/Game/BP_GameMode` (`GameplayStatics.GetGameMode`)))
        (`/Game/BP_GameMode.CandyObtainedEvent` _asbp_game_mode)
        (`self.CandyBag_WhupWhup`)
        (else
          (`SceneComponent.K2_AddWorldOffset` _candy1 (* (`KismetMathLibrary.Normal` _returnvalue) (`KismetMathLibrary.Conv_DoubleToVector` (- (`self.BaseDragSpeed`) _returnvalue_2)) (/ 1 (`GameUserSettings.GetFramePace`))) false false))))))

(event `CandyBag_WhupWhup`
  (bind _candybag (`self.CandyBag`))
  (bind (_direction _newtrack_0) (`Timeline|Bag_whup_whup` :!via `PlayFromStart`)
    (:`Update`
      (`SceneComponent.SetRelativeScale3D` _candybag (+ _newtrack_0 (`self.BagScale`)))
      (`MeshComponent.SetScalarParameterValueOnMaterials` _candybag "Emit" (* _newtrack_0 0.5)))))

(fn `UserConstructionScript`)