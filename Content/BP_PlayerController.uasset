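; Player controller that switches the player between two tools, a mouse-driven bat and an axis-driven vacuum cleaner.
; While active, the bat follows the cursor each tick, its deprojected ray scaled by BatDepth onto a plane perpendicular to X.
; Otherwise, movement axes slide the vacuum within fixed X/Y bounds.
; ChangeAction swaps tools by teleporting them to preset positions and toggling the vacuum sound, while Enable/Disable start or stop control.
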(event `self.ReceiveBeginPlay`
  (bind _returnvalue (`GameplayStatics.GetActorOfClass` "/Game/BP_Bat.BP_Bat_C"))
  (set `self.Bat` _returnvalue)
  (bind _returnvalue_2 (`GameplayStatics.GetActorOfClass` "/Game/BP_VacuumCleaner.BP_VacuumCleaner_C"))
  (set `self.VacuumCleaner` _returnvalue_2))

(event `Disable`
  (set `self.isGameStarted` false)
  (`self.DisableBat`)
  (`self.DisableVacuumCleaner`))

(event `Enable`
  (set `self.isGameStarted` true)
  (`self.EnableBat`))

(event `self.ReceiveTick`
  (params (DeltaSeconds :type "Float (single-precision)"))
  (bind (_locationx _locationy) (`self.GetMousePosition`))
  (bind (_worldlocation _worlddirection) (`self.DeprojectScreenPositionToWorld` _locationx _locationy))
  (if (`self.IsBatActive`)
    (bind _newparam1 (`self.BatOffset` _worlddirection))
    (`self.K2_SetActorLocation` (`self.Bat`) (+ _worldlocation _newparam1 (0.0 50.0 -50.0)) false false)))

(event `InputAxis|ActionMoveX`
  (params (AxisValue :type "Float (single-precision)"))
  (bind _returnvalue (* AxisValue -1.0 (`self.VacuumCleanerSpeed`)))
  (if (`self.IsBatActive`)
    _
    (elif (`KismetMathLibrary.InRange_FloatFloat` (+ (.y (`self.K2_GetActorLocation` (`self.VacuumCleaner`))) _returnvalue) -700.0 740.0 false false)
      (`self.K2_AddActorWorldOffset` (`self.VacuumCleaner`) (`KismetMathLibrary.MakeVector` 0.0 _returnvalue) true false))))

(event `InputAxis|ActionMoveY`
  (params (AxisValue :type "Float (single-precision)"))
  (bind _returnvalue (* AxisValue -1.0 (`self.VacuumCleanerSpeed`)))
  (if (`self.IsBatActive`)
    _
    (elif (`KismetMathLibrary.InRange_FloatFloat` (+ (.x (`self.K2_GetActorLocation` (`self.VacuumCleaner`))) _returnvalue) -140.0 1200.0 false false)
      (`self.K2_AddActorWorldOffset` (`self.VacuumCleaner`) (`KismetMathLibrary.MakeVector` _returnvalue) true false))))

(event `InputAction|ChangeAction`
  (params (Key :type "Key Structure"))
  (:`Pressed`
    (if (`self.IsBatActive`)
      (`self.DisableBat`)
      (`self.EnableVacuumCleaner`)
      (else
        (`self.DisableVacuumCleaner`)
        (`self.EnableBat`)))))

(fn `BatOffset`
  (params (NewParam :type "Vector Structure"))
  (returns (NewParam1 :type "Vector Structure"))
  (return (* NewParam (/ (`self.BatDepth`) (`KismetMathLibrary.Dot_VectorVector` NewParam (-1.0 0.0 0.0))))))

(fn `DisableBat`
  (`self.K2_SetActorLocation` (`self.Bat`) (320.0 -1000.0 520.0) false true)
  (set `self.IsBatActive` false))

(fn `DisableVacuumCleaner`
  (`self.K2_SetActorLocation` (`self.VacuumCleaner`) (-2000.0 -800.0 270.0) false true)
  (`AudioComponent.Stop` (`self.VacuumCleanerSound`)))

(fn `EnableBat`
  (set `self.IsBatActive` true))

(fn `EnableVacuumCleaner`
  (`self.K2_SetActorLocation` (`self.VacuumCleaner`) (1000.0 0.0 270.0) false true)
  (bind _returnvalue (`GameplayStatics.CreateSound2D` "/Game/Sound/Vacuum_Cleaner_Working.Vacuum_Cleaner_Working" 1.0 1.0 0.0 null))
  (bind _output_get (set `self.VacuumCleanerSound` _returnvalue))
  (`AudioComponent.Play` _output_get 0.0))

(fn `UserConstructionScript`)