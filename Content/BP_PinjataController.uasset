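; Controller that runs a piñata level, spawning piñatas at left, center and right spawn points and deciding the win or loss.
; StartPlay chains a LifeCycle macro into staggered, looping waves through its Exit and Finish outputs.
; Each cycle spawns a piñata with randomized scale and colors, later raises its ceiling, destroys it and decrements PinatasLeft.
; At zero left, Tick compares game mode candy to the target and shows the congratulation or oops widget.
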(event `self.ReceiveBeginPlay`)

(event `Event StartPlay`
  (`self.LifeCycle` 1.0 (`self.SpawnPointLeft`)
    (:`Exit`
      (`self.LifeCycle` 3.0 (`self.SpawnPointRight`)))
    (:`Finish`
      (`self.LifeCycle` 2.0 (`self.SpawnPointCenter`) :!label _label
        (:`Exit`
          (`KismetSystemLibrary.Delay` 1.0)
          (`self.LifeCycle` 2.0 (`self.SpawnPointRight`) :!label _label_2
            (:`Finish`
              (`KismetSystemLibrary.Delay` 2.0)
              (goto _label_2))))
        (:`Finish`
          (`self.LifeCycle` 1.0 (`self.SpawnPointLeft`)
            (:`Finish`
              (goto _label))))))))

(event `self.ReceiveTick`
  (params (DeltaSeconds :type "Float (single-precision)"))
  (if (<= (`self.Pinatas_left`) 0)
    (`KismetSystemLibrary.Delay` 2.0)
    (bind _asbp_game_mode (cast `/Game/BP_GameMode` (`GameplayStatics.GetGameMode`)))
    (if (>= (`/Game/BP_GameMode.CandyObtained` _asbp_game_mode) (`/Game/BP_GameMode.TargetCandyValue` _asbp_game_mode))
      (`KismetSystemLibrary.PrintString` "WIN")
      (bind _returnvalue (`|CreateWidget` "/Game/UI/WB_Congratulation.WB_Congratulation_C"))
      (`UserWidget.AddToViewport` _returnvalue 0)
      (else
        (`KismetSystemLibrary.PrintString` "LOOSE")
        (bind _returnvalue_2 (`|CreateWidget` "/Game/UI/WB_Oops.WB_Oops_C"))
        (`UserWidget.AddToViewport` _returnvalue_2 0)))))

(fn `RandomColorAndScale`
  (params (self2 :type "/Game/Pinjata Object Reference") (NewScale_Y :type "Float (double-precision)") (NewScale_X :type "Float (double-precision)") (NewScale_Z :type "Float (double-precision)"))
  (bind _pinjata (`/Game/Pinjata.Pinjata` self2))
  (`SceneComponent.SetWorldScale3D` _pinjata (`KismetMathLibrary.MakeVector` NewScale_X NewScale_Y NewScale_Z))
  (`MeshComponent.SetScalarParameterValueOnMaterials` _pinjata "RandomColor" (`KismetMathLibrary.RandomFloatInRange` 0.0 1.0))
  (`MeshComponent.SetScalarParameterValueOnMaterials` _pinjata "RandomColor2" (`KismetMathLibrary.RandomFloatInRange` 0.0 1.0))
  (`MeshComponent.SetScalarParameterValueOnMaterials` _pinjata "RandomColor3" (`KismetMathLibrary.RandomFloatInRange` 0.0 1.0)))

(fn `UserConstructionScript`)